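; Energy shield actor that destroys overlapping actors whose class is in ActorsToAbsorb, then fires OnShieldAbsorb.
; Each absorb plays a sound and a timeline pulse of the dynamic material's Pow parameter.
; Activate and Deactivate toggle AbsorbtionZone collision and play or reverse a scale timeline at a given rate.
; DefaultActive sets initial collision and Shield mesh scale at construction, whereas the timeline scales the whole actor.
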(event `self.ReceiveBeginPlay`)

(event `self.AbsorbtionZone.OnComponentBeginOverlap`
  (params (OverlappedComponent :type "PrimitiveComponent Object Reference") (OtherActor :type "Actor Object Reference") (OtherComp :type "PrimitiveComponent Object Reference") (OtherBodyIndex :type Integer) (bFromSweep :type Boolean) (SweepResult :type "HitResult Structure (by ref)"))
  (if (`KismetArrayLibrary.Array_Contains` (`self.ActorsToAbsorb`) (`GameplayStatics.GetObjectClass` OtherActor))
    (`self.K2_DestroyActor` OtherActor)
    (`self.PulseShield`)
    (`self.OnShieldAbsorb`)))

(event `PulseShield`
  (`GameplayStatics.PlaySoundAtLocation` "/Game/EnergyShield/Audio/Cues/Cue_Shield_Absorb.Cue_Shield_Absorb" (`self.K2_GetActorLocation`) (struct) 1.0 1.0 0.0 null null null null)
  (`self.ShieldMaterial`
    (:`then`
      (bind (_direction _shieldpoweralpha) (`Timeline|PulseShieldTimeline` :!via `PlayFromStart`)
        (:`Update`
          (`MaterialInstanceDynamic.SetScalarParameterValue` (`self.ShieldMaterial`) "Pow" (`KismetMathLibrary.Lerp` (`self.ShieldMaterialDefaultPower`) 0.1 _shieldpoweralpha)))))
    (:`else`)))

(event `Activate`
  (params (PlayRate :type "Float (double-precision)" :default 1.0))
  (`self.ExpandShield` PlayRate)
  (`PrimitiveComponent.SetCollisionEnabled` (`self.AbsorbtionZone`) "QueryOnly"))

(event `Deactivate`
  (params (PlayRate :type "Float (double-precision)" :default 1.0))
  (`self.ShrinkShield` PlayRate)
  (`PrimitiveComponent.SetCollisionEnabled` (`self.AbsorbtionZone`) "NoCollision"))

(event `ExpandShield`
  (params (PlayRate :type "Float (double-precision)" :default 1.0))
  (`TimelineComponent.SetPlayRate` (`self.ExpandTimeline`) PlayRate)
  (bind (_direction _scalealpha) (`Timeline|ExpandTimeline` :!via `PlayFromStart` :!label _label)
    (:`Update`
      (`self.SetActorRelativeScale3D` (`KismetMathLibrary.Conv_DoubleToVector` (`KismetMathLibrary.Lerp` 0.0 1.0 _scalealpha))))))

(event `ShrinkShield`
  (params (PlayRate :type "Float (double-precision)" :default 1.0))
  (`TimelineComponent.SetPlayRate` (`self.ExpandTimeline`) PlayRate)
  (goto _label :!via `Reverse`))

(fn `UserConstructionScript`
  (`|ExecutionSequence`
    (:`then_0`
      ;[1 1 1] Setup dyamic material instance
      (bind _returnvalue (`PrimitiveComponent.CreateDynamicMaterialInstance` (`self.Shield`) 0 "/Game/EnergyShield/Material/M_EnergyShield.M_EnergyShield" "None"))
      (bind _output_get (set `self.ShieldMaterial` _returnvalue))
      (bind _returnvalue_2 (`MaterialInstanceDynamic.K2_GetScalarParameterValue` _output_get "Pow"))
      (set `self.ShieldMaterialDefaultPower` _returnvalue_2))
    (:`then_1`
      ;[1 1 1] Initial shield state
      (`SceneComponent.SetRelativeScale3D` (`self.Shield`) (`KismetMathLibrary.SelectVector` (1.0 1.0 1.0) (0.0 0.0 0.0) (`self.DefaultActive`)))
      (`PrimitiveComponent.SetCollisionEnabled` (`self.AbsorbtionZone`) (select `bool` (`self.DefaultActive`) :`false` "NoCollision" :`true` "QueryOnly" :!type "ECollisionEnabled Enum")))))